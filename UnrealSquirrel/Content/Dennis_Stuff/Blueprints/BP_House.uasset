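; BP_House is a placeable house actor with a mesh and a point light, configured per instance.
; Its construction script creates a dynamic instance of M_House, sets the Colour parameter from the Colour variable and applies it to the mesh.
; The same script sets the point light's shadow casting and visibility from exposed-style variables.
; The event graph holds no gameplay logic.
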(event EventBeginPlay)

(event Collision|EventActorBeginOverlap
  (params (OtherActor :type Actor%20Object%20Reference)))

(event EventTick
  (params (DeltaSeconds :type Float%20%28single-precision%29)))

(fn ConstructionScript
  (bind _returnvalue (Rendering|Material|CreateDynamicMaterialInstance "/Game/Dennis_Stuff/Meshes/House/M_House.M_House" "None" :!class /Script/Engine.KismetMaterialLibrary))
  (Rendering|Material|SetVectorParameterValue _returnvalue "Colour" (Variables|Default|GetColour) :!class /Script/Engine.MaterialInstanceDynamic)
  (Rendering|Material|SetMaterial (Variables|Default|GetMesh) 0 _returnvalue)
  (Rendering|Components|Light|SetCastShadows (Variables|Default|GetPointLight) (Variables|Default|GetLight_Cast_Shadow))
  (Rendering|SetVisibility (Variables|Default|GetPointLight) (Variables|Default|GetLight_Visibility) false))