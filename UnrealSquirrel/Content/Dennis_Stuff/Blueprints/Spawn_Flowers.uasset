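; Construction-script scatterer that covers static world geometry with flower planes as instances around the actor.
; For each of NR attempts, it line traces downward between seeded random offsets scaled by Range, drawn lopsidedly toward negative X and Y.
; Each hit adds a raised, upright instance with an unseeded random yaw.
; The Flower index picks one of five materials for the whole instanced component; a random material switch is left unconnected.
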(event EventBeginPlay)

(event Collision|EventActorBeginOverlap
  (params (OtherActor :type Actor%20Object%20Reference)))

(event EventTick
  (params (DeltaSeconds :type Float%20%28single-precision%29)))

(fn ConstructionScript
  (bind _returnvalue (Transformation|GetActorLocation))
  (bind _range (Variables|Default|GetRange))
  (bind _key (Variables|Default|GetKey))
  (bind _plane (Variables|Default|GetPlane))
  (bind _returnvalue_2 (* _range -1e+01))
  (bind _returnvalue_3 (Math|Random|RandomFloatinRangefromStream _returnvalue_2 _range _key))
  (bind _returnvalue_4 (Math|Random|RandomFloatinRangefromStream _returnvalue_2 _range _key))
  (for _index (range 0 (Variables|Default|GetNR))
    (bind (_outhit _returnvalue_5) (Collision|LineTraceForObjects (+ _returnvalue (Math|Vector|MakeVector _returnvalue_4 _returnvalue_3 1e+04)) (+ _returnvalue (Math|Vector|MakeVector _returnvalue_4 _returnvalue_3 -1e+04)) (Utilities|Array|MakeArray "ObjectTypeQuery1") false 0 "ForOneFrame"))
    (if _returnvalue_5
      (Class|InstancedStaticMeshComponent|AddInstanceWorldSpace _plane (Math|Transform|MakeTransform (+ (.Location (Collision|BreakHitResult _outhit)) "0, 0,45.000000") (Math|Rotator|MakeRotator 9e+01 0.0 (Math|Random|RandomFloatinRange 0.0 1.8e+02)) "1,1,1"))
      (Rendering|Material|SetMaterial _plane 0 (Utilities|Array|Get(acopy) (Utilities|Array|MakeArray "/Game/Dennis_Stuff/Materials/M_Flower.M_Flower" "/Game/Dennis_Stuff/Materials/MI_Flower_2.MI_Flower_2" "/Game/Dennis_Stuff/Materials/M_Flower_Inst.M_Flower_Inst" "/Game/Dennis_Stuff/Materials/M_Flower_Inst1.M_Flower_Inst1" "/Game/Dennis_Stuff/Materials/M_Flower_Inst2.M_Flower_Inst2") (Variables|Default|GetFlower))))))