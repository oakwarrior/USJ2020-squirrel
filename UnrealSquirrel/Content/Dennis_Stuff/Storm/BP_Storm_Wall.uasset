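; BP_Storm_Wall is a moving storm hazard that creeps along +X on a looping timer whenever the Player is not on the ground.
; When a FlyingPawn enters the storm, a looping fatigue timer plays SFX, updates the sound manager and kills the player at the limit.
; A cloud overlap changes the season, while storm post-process transitions are only debug prints.
; ResetSession restores the start position and fatigue count, but nothing clears the fatigue timer.
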(event OnComponentBeginOverlap(StormCollision)
  (params (OverlappedComponent :type Primitive%20Component%20Object%20Reference) (OtherActor :type Actor%20Object%20Reference) (OtherComp :type Primitive%20Component%20Object%20Reference) (OtherBodyIndex :type Integer) (bFromSweep :type Boolean) (SweepResult :type Hit%20Result%20Structure%20%28by%20ref%29))
  (Utilities|Casting|CastToFlyingPawn OtherActor)
  (Development|PrintString "SHOULD BE IN STORM POST PROCESS")
  (Utilities|Time|SetTimerbyFunctionName 0 "StormFatigue" 0.5 true))

(event OnComponentBeginOverlap(AfterStormCollision)
  (params (OverlappedComponent :type Primitive%20Component%20Object%20Reference) (OtherActor :type Actor%20Object%20Reference) (OtherComp :type Primitive%20Component%20Object%20Reference) (OtherBodyIndex :type Integer) (bFromSweep :type Boolean) (SweepResult :type Hit%20Result%20Structure%20%28by%20ref%29))
  (Utilities|Casting|CastToFlyingPawn OtherActor)
  (Development|PrintString "SHOULD BE IN AFTER STORM POST PROCESS"))

(event OnComponentBeginOverlap(Clouds_01)
  (params (OverlappedComponent :type Primitive%20Component%20Object%20Reference) (OtherActor :type Actor%20Object%20Reference) (OtherComp :type Primitive%20Component%20Object%20Reference) (OtherBodyIndex :type Integer) (bFromSweep :type Boolean) (SweepResult :type Hit%20Result%20Structure%20%28by%20ref%29))
  (Utilities|Casting|CastToFlyingPawn OtherActor)
  (Development|PrintString "SPRING PLIS")
  (Default|ChangeSeason (Variables|Default|GetSeasonChangeComponent) "NewEnumerator1"))

(event Custom|MoveForward
  (if (not (Variables|/Game/Blueprints/Character/MoveComponent.MoveComponent_C|GetIsOnGround (Variables|/Game/Blueprints/Character/FlyingPawn.FlyingPawn_C|GetMoveComponent (Variables|Default|GetPlayer))))
    (Transformation|SetActorLocation (+ (Transformation|GetActorLocation self) "5.000000, 0, 0") false false)))

(event Custom|StormFatigue
  (CallFunction|PlaySFX "NewEnumerator6")
  (bind _result (Math|Integer|IncrementInt (Variables|Default|GetStormFatigueCount))
    (:%20%20
      (Development|PrintString (Utilities|String|ToString(Integer) _result))
      (if (>= _result 10)
        (Variables|Default|SetStormFatigueCount 0)
        (CallFunction|KillPlayer)
        (else
          (Default|NotifyFatigueUpdated (CallFunction|GetSoundManager) (/ (Math|Conversions|ToFloat(Integer) _result) 1e+01)))))))

(event Custom|ResetSession
  (Variables|Default|SetStormFatigueCount 0)
  (Transformation|SetActorLocation (Variables|Default|GetStartingPosition) false false))

(event EventBeginPlay
  (Utilities|Time|SetTimerbyFunctionName 0 "MoveForward" 0.02 true)
  (Variables|Default|SetStartingPosition (Transformation|GetActorLocation)))

(fn ConstructionScript)