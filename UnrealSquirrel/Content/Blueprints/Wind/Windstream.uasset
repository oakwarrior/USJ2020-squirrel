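; Windstream actor: a spline-shaped wind current that affects FlyingPawns overlapping it.
; The construction script builds a spline mesh component along each spline segment.
; Overlap begin and end add or remove the stream in the pawn MoveComponent's AffectingWindstreams list, with debug prints.
; A helper interpolates distance along the spline nearest a location; its only use here is disconnected legacy logic that set pawn wind directly.
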(event EventBeginPlay)

(event EventTick
  (params (DeltaSeconds :type Float%20%28single-precision%29)))

(event Collision|EventActorBeginOverlap
  (params (OtherActor :type Actor%20Object%20Reference))
  (bind _asflying_pawn (Utilities|Casting|CastToFlyingPawn OtherActor))
  (Utilities|Array|AddUnique (Variables|/Game/Blueprints/Character/MoveComponent.MoveComponent_C|GetAffectingWindstreams (Variables|/Game/Blueprints/Character/FlyingPawn.FlyingPawn_C|GetMoveComponent _asflying_pawn)) self)
  (Development|PrintString "BEGIN WINDSTREAM" true true "(R=0.000000,G=0.000000,B=0.000000,A=1.000000)" 4.0))

(event Collision|EventActorEndOverlap
  (params (OtherActor :type Actor%20Object%20Reference))
  (bind _asflying_pawn (Utilities|Casting|CastToFlyingPawn OtherActor))
  (Utilities|Array|RemoveItem (Variables|/Game/Blueprints/Character/MoveComponent.MoveComponent_C|GetAffectingWindstreams (Variables|/Game/Blueprints/Character/FlyingPawn.FlyingPawn_C|GetMoveComponent _asflying_pawn)) self)
  (Development|PrintString "END WINDSTREAM" true true "(R=0.000000,G=0.000000,B=0.000000,A=1.000000)" 4.0))

(fn ConstructionScript
  (bind _spline (Variables|Default|GetSpline))
  (for _index (range 0 (- (Spline|GetNumberOfSplinePoints (Variables|Default|GetSpline)) 2))
    (bind _returnvalue (AddComponent|AddSplineMeshComponent true))
    (Transformation|AttachComponentToComponent _returnvalue (Variables|Default|GetRoot) "None" "KeepRelative" "KeepRelative" "KeepRelative" true)
    (SplineMesh|SetStartandEnd _returnvalue (.Location (Spline|GetLocationandTangentatSplinePoint _spline _index "Local")) (.Tangent (Spline|GetLocationandTangentatSplinePoint _spline _index "Local")) (.Location (Spline|GetLocationandTangentatSplinePoint _spline (+ _index 1) "Local")) (.Tangent (Spline|GetLocationandTangentatSplinePoint _spline (+ _index 1) "Local")) true :!class /Script/Engine.SplineMeshComponent)))

(fn FindDistanceAlongSplineClosesttoWorldLocation
  (params (WorldLocation :type Vector))
  (bind _spline (Variables|Default|GetSpline))
  (bind _returnvalue (Class|SplineComponent|FindInputKeyClosesttoWorldLocation _spline WorldLocation))
  (bind _returnvalue_2 (Math|Float|Truncate _returnvalue))
  (bind _returnvalue_3 (Spline|GetDistanceAlongSplineatSplinePoint _spline _returnvalue_2))
  (return (+ _returnvalue_3 (* (- (Spline|GetDistanceAlongSplineatSplinePoint _spline (Math|Float|Truncate (+ _returnvalue 1.0))) _returnvalue_3) (- _returnvalue (Math|Conversions|ToFloat(Integer) _returnvalue_2))))))