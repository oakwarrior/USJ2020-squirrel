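; Component that switches the game's current season through ChangeSeason.
; It stores the new season and passes it to the player's PlayerInteractionComponent.
; It then finds every Coin actor, calls Change with whether the season matches one specific enum value, and clears its picked-up flag.
; A disconnected branch that hid actors not matching the season remains unused.
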(event EventBeginPlay)

(event EventTick
  (params (DeltaSeconds :type Float%20%28single-precision%29)))

(fn ChangeSeason
  (params (NewSeason :type EGameSeason%20Enum :default "NewEnumerator0"))
  (bind _output_get (Variables|Default|SetSeason NewSeason))
  (Default|HandleSeasonChange (Variables|/Game/Blueprints/Character/FlyingPawn.FlyingPawn_C|GetPlayerInteractionComponent (CallFunction|GetPlayer)) _output_get)
  (bind _outactors (Actor|GetAllActorsOfClass "/Game/Blueprints/Simon_Test/Coin.Coin_C"))
  (for _array_element _outactors
    (Default|Change _array_element (Utilities|Enum|Equal(Enum) _output_get "NewEnumerator1"))
    (Variables|/Game/Blueprints/Simon_Test/Coin.Coin_C|SetIsPickedUp _array_element false)))