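; PawnPlayer is a player pawn driven by physics on its Sphere, flying constantly forward and possessed by player 0 on BeginPlay.
; The MoveForward axis overwrites linear velocity along actor forward, but its input is zeroed before clamping, so speed stays at the minimum.
; MoveRight, MouseX and MouseY all add roll torque around the forward vector at different strengths.
; Tick applies opposing torque proportional to angular velocity to damp spin.
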(event EventBeginPlay
  (Pawn|Possess (Game|GetPlayerController 0) self))

(event Collision|EventActorBeginOverlap
  (params (OtherActor :type Actor%20Object%20Reference)))

(event EventTick
  (params (DeltaSeconds :type Float%20%28single-precision%29))
  (bind _sphere (Variables|Default|GetSphere))
  (Class|PrimitiveComponent|AddTorqueinRadians _sphere (/ (Math|Vector|NegateVector (Class|PrimitiveComponent|GetPhysicsAngularVelocityinRadians _sphere "None")) 2e+01) "None" true))

(event Input|AxisEvents|InputAxisMouseX
  (params (AxisValue :type Float%20%28single-precision%29))
  (Class|PrimitiveComponent|AddTorqueinRadians (Variables|Default|GetSphere) (Math|Vector|Lerp(Vector) "0, 0, 0" (* (Transformation|GetActorForwardVector) (* AxisValue 15.0)) 1.0) "None" true))

(event Input|AxisEvents|InputAxisMouseY
  (params (AxisValue :type Float%20%28single-precision%29))
  (Class|PrimitiveComponent|AddTorqueinRadians (Variables|Default|GetSphere) (Math|Vector|Lerp(Vector) "0, 0, 0" (* (Transformation|GetActorForwardVector) (* AxisValue 3e+01)) 1.0) "None" true))

(event Input|AxisEvents|InputAxisMoveForward
  (params (AxisValue :type Float%20%28single-precision%29))
  (bind _sphere (Variables|Default|GetSphere))
  (bind _returnvalue (Physics|GetPhysicsLinearVelocity _sphere "None"))
  (Physics|SetPhysicsLinearVelocity _sphere (Math|Vector|Lerp(Vector) _returnvalue (* (Transformation|GetActorForwardVector) (Math|Float|Clamp(Float) (* AxisValue 0.0) 4e+03 1e+04)) 1.0) false "None"))

(event Input|AxisEvents|InputAxisMoveRight
  (params (AxisValue :type Float%20%28single-precision%29))
  (Class|PrimitiveComponent|AddTorqueinRadians (Variables|Default|GetSphere) (Math|Vector|Lerp(Vector) "0, 0,0.000000" (* (Transformation|GetActorForwardVector) (* AxisValue 4e+01)) 1.0) "None" true))

(fn ConstructionScript)