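; Player interaction component that handles NPC focus, coin collection and start, restart and session reset.
; A forward sphere trace sets the player's focused NPC and toggles its outline, and Interact triggers that NPC.
; Collected coins are tracked for reset, and DropCoin pops the oldest beside the player with a random physics impulse.
; ResetGame clears points, unhides coins, returns the player to PlayerStart, revives them and resets the storm wall.
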(event Custom|IncrementCoins
  (params (Coin :type Coin%20Object%20Reference))
  (Math|Integer|IncrementInt (Variables|Default|Getpoints)
    (:%20%20
      (Utilities|Array|AddUnique (Variables|Default|GetCoinsTakenArray) Coin))))

(event Custom|DropCoin
  (bind _returnvalue (Math|Random|RandomUnitVector))
  (bind _coinstakenarray (Variables|Default|GetCoinsTakenArray))
  (bind _output (Utilities|Array|Get(acopy) _coinstakenarray))
  (bind _cube1 (Variables|/Game/Blueprints/Simon_Test/Coin.Coin_C|GetCube1 _output))
  (if (> (Utilities|Array|Length _coinstakenarray) 0)
    (Rendering|SetActorHiddenInGame _output false)
    (Transformation|SetActorLocation _output (+ (Transformation|GetActorLocation (Variables|Default|Getplayer)) (* (Math|Vector|Normalize (Math|Vector|MakeVector (.x _returnvalue) (.y _returnvalue) 0.0)) 5e+01)) false true)
    (Physics|SetSimulatePhysics _cube1 true)
    (Physics|AddImpulse _cube1 (+ (* (Transformation|GetActorUpVector _output) 1e+03) (* (Transformation|GetActorRightVector _output) (Math|Random|RandomFloatinRange -8e+02 8e+02))) "None" true)
    (Utilities|Array|RemoveIndex _coinstakenarray)))

(event Custom|ResetGame
  (Variables|Default|Setpoints 0)
  (for _array_element (Variables|Default|GetCoinsTakenArray)
    (Rendering|SetActorHiddenInGame _array_element false))
  (bind _outactors (Actor|GetAllActorsOfClass "/Script/Engine.PlayerStart"))
  (Transformation|SetActorLocationAndRotation (Variables|Default|Getplayer) (Transformation|GetActorLocation (Utilities|Array|Get(acopy) _outactors)) (Transformation|GetActorRotation (Utilities|Array|Get(acopy) _outactors)))
  (Default|SetIsDead (Variables|Default|Getplayer) false)
  (Default|ToggleFlying (Variables|/Game/Blueprints/Character/FlyingPawn.FlyingPawn_C|GetMoveComponent (Variables|Default|Getplayer)) false)
  (bind _outactors_2 (Actor|GetAllActorsOfClass "/Game/Dennis_Stuff/Storm/BP_Storm_Wall.BP_Storm_Wall_C"))
  (Default|ResetSession (Utilities|Array|Get(acopy) _outactors_2))
  (Variables|Default|SetDEATH false))

(event Custom|Interact
  (bind _player (Variables|Default|Getplayer))
  (bind _currentfocusnpc (Variables|/Game/Blueprints/Character/FlyingPawn.FlyingPawn_C|GetCurrentFocusNPC _player))
  (Utilities|IsValid _currentfocusnpc
    (:Is%20Valid
      (Default|Interacedwith _currentfocusnpc))))

(event Custom|AnyKeyCheck
  (bind _player (Variables|Default|Getplayer))
  (if (Variables|Default|GetDEATH)
    (Default|RestartGame (Variables|Default|GetendgameWidget))
    (else
      (Utilities|IsValid _player
        (:Is%20Valid
          (Default|StartGame (Variables|/Game/Blueprints/Character/FlyingPawn.FlyingPawn_C|GetStartScreen _player)))))))

(event EventTick
  (params (DeltaSeconds :type Float%20%28single-precision%29)))

(event EventBeginPlay)

(fn TraceforInteraction
  (bind _player (Variables|Default|Getplayer))
  (bind _player_2 (Variables|Default|Getplayer))
  (bind _skeletalmesh (Variables|/Game/Blueprints/Character/FlyingPawn.FlyingPawn_C|GetSkeletalMesh _player))
  (bind _returnvalue (Transformation|GetWorldLocation _skeletalmesh))
  (bind _returnvalue_2 (+ _returnvalue "0, 0,90.000000"))
  (bind _outhit (Collision|SphereTraceForObjects _returnvalue_2 (+ _returnvalue_2 (* (Math|Vector|GetForwardVector (Variables|/Game/Blueprints/Character/FlyingPawn.FlyingPawn_C|GetCamera _player)) 5e+02)) 2e+02 (Utilities|Array|MakeArray (Utilities|Enum|LiteralenumEObjectTypeQuery "ObjectTypeQuery3")) false (Utilities|Array|MakeArray (Variables|Default|Getplayer)) "None"))
  (bind _ascharacter_npc (Utilities|Casting|CastToCharacterNPC (.hitactor _outhit))
    (:then
      (if (== _ascharacter_npc (Variables|/Game/Blueprints/Character/FlyingPawn.FlyingPawn_C|GetCurrentFocusNPC _player_2))
        (Default|EnableOutline _ascharacter_npc)
        (else
          (Utilities|IsValid (Variables|/Game/Blueprints/Character/FlyingPawn.FlyingPawn_C|GetCurrentFocusNPC _player_2)
            (:Is%20Valid
              (Default|DisableOutline (Variables|/Game/Blueprints/Character/FlyingPawn.FlyingPawn_C|GetCurrentFocusNPC _player_2)))
            (:Is%20Not%20Valid
              _))
          (bind _output_get (Variables|/Game/Blueprints/Character/FlyingPawn.FlyingPawn_C|SetCurrentFocusNPC _player_2 _ascharacter_npc))
          (Default|EnableOutline _output_get)))
      (return))
    (:CastFailed
      (Utilities|IsValid (Variables|/Game/Blueprints/Character/FlyingPawn.FlyingPawn_C|GetCurrentFocusNPC _player_2)
        (:Is%20Valid
          (Default|DisableOutline (Variables|/Game/Blueprints/Character/FlyingPawn.FlyingPawn_C|GetCurrentFocusNPC _player_2)))
        (:Is%20Not%20Valid
          _))
      (Variables|/Game/Blueprints/Character/FlyingPawn.FlyingPawn_C|SetCurrentFocusNPC _player_2 0))))

(fn HandleSeasonChange
  (params (NewSeason :type EGameSeason%20Enum :default "NewEnumerator0"))
  (Variables|Default|SetSeason NewSeason)
  (switch Utilities|FlowControl|Switch|SwitchonEGameSeason NewSeason))