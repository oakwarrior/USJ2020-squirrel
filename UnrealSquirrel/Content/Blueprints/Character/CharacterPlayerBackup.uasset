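; Player character with walking, jumping and a glide toggled by pressing Jump midair, plus NPC interaction, coin counting and start/dialogue widgets.
; Gliding uses Flying mode with a manual per-tick update: input tilts the mesh, pitch drives speed, and velocity blends gravity with facing before a swept offset.
; Interact line-traces for NPCs and opens placeholder test dialogue.
; MoveRight lacks a Flying branch, leaving glide steering unfed, and UpdateWind is never called.
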(event Custom|AddDialogueBox
  (Utilities|IsValid (Variables|Default|GetDialogueBox)
    (:Is%20Valid
      (Default|OpenDialogueWidget (Variables|Default|GetDialogueBox) "This text is for testing! and testing is what i'll DO!"))
    (:Is%20Not%20Valid
      (bind _returnvalue (UserInterface|CreateWidget "/Game/Blueprints/Simon_Test/DialogueWidget.DialogueWidget_C"))
      (Variables|Default|SetDialogueBox _returnvalue)
      (UserInterface|Viewport|AddtoViewport _returnvalue 0)
      (Default|OpenDialogueWidget _returnvalue "This text is for testing! and testing is what i'll DO!"))))

(event Custom|IncrementCoins
  (Math|Integer|IncrementInt (Variables|Default|Getpoints)))

(event EventBeginPlay
  (bind _returnvalue (UserInterface|CreateWidget "/Game/Blueprints/Simon_Test/StartGame.StartGame_C"))
  (UserInterface|Viewport|AddtoViewport _returnvalue 0)
  (Variables|Default|SetStartScreen _returnvalue))

(event Collision|EventActorBeginOverlap
  (params (OtherActor :type Actor%20Object%20Reference)))

(event EventTick
  (params (DeltaSeconds :type Float%20%28single-precision%29))
  (CallFunction|UpdateGlide))

(event Input|ActionEvents|InputActionJump
  (params (Key :type Key%20Structure :default "None"))
  (:Pressed
    (switch Utilities|FlowControl|Switch|SwitchonEMovementMode (Variables|/Script/Engine.CharacterMovementComponent|GetMovementMode (Variables|Character|GetCharacterMovement))
      (:MOVE_Walking
        (Character|Jump))
      (:MOVE_Falling
        (CallFunction|SetFlying true))
      (:MOVE_Flying
        (CallFunction|SetFlying false))))
  (:Released
    (Character|StopJumping)))

(event Input|ActionEvents|InputActionAnyInputKey
  (params (Key :type Key%20Structure :default "None"))
  (bind _dialoguebox (Variables|Default|GetDialogueBox))
  (:Pressed
    (Default|StartGame (Variables|Default|GetStartScreen))
    (Utilities|IsValid _dialoguebox
      (:Is%20Valid
        (Default|CompleteText _dialoguebox)))))

(event Input|ActionEvents|InputActionInteract
  (params (Key :type Key%20Structure :default "None"))
  (:Pressed
    (CallFunction|AddDialogueBox)))

(event Input|ActionEvents|InputActionInteract
  (params (Key :type Key%20Structure :default "None"))
  (bind _mesh (Variables|Character|GetMesh))
  (bind _returnvalue (Transformation|GetWorldLocation _mesh))
  (bind _returnvalue_2 (+ _returnvalue "0, 0,90.000000"))
  (:Pressed
    (bind _outhit (Collision|LineTraceForObjects _returnvalue_2 (+ _returnvalue_2 (* (Math|Vector|GetForwardVector (Variables|Default|GetCapsuleComponent)) 7e+02)) (Utilities|Array|MakeArray (Utilities|Enum|LiteralenumEObjectTypeQuery "ObjectTypeQuery2")) false (Utilities|Array|MakeArray self) "ForDuration"))
    (bind _ascharacter_npc (Utilities|Casting|CastToCharacterNPC (.hitactor _outhit)))
    (Default|Interacedwith _ascharacter_npc)))

(event Input|AxisEvents|InputAxisMouseX
  (params (AxisValue :type Float%20%28single-precision%29))
  (Pawn|Input|AddControllerYawInput AxisValue))

(event Input|AxisEvents|InputAxisMouseY
  (params (AxisValue :type Float%20%28single-precision%29))
  (switch Utilities|FlowControl|Switch|SwitchonEMovementMode (Variables|/Script/Engine.CharacterMovementComponent|GetMovementMode (Variables|Character|GetCharacterMovement))
    (:MOVE_Walking
      _)
    (:MOVE_Falling
      _))
  (Pawn|Input|AddControllerPitchInput AxisValue))

(event Input|AxisEvents|InputAxisMoveForward
  (params (AxisValue :type Float%20%28single-precision%29))
  (switch Utilities|FlowControl|Switch|SwitchonEMovementMode (Variables|/Script/Engine.CharacterMovementComponent|GetMovementMode (Variables|Character|GetCharacterMovement))
    (:MOVE_Walking
      (Pawn|Input|AddMovementInput (Math|Vector|GetForwardVector (Math|Rotator|MakeRotator 0.0 0.0 (.Yaw (Math|Rotator|BreakRotator (Pawn|GetControlRotation :!class /Script/Engine.Pawn))))) AxisValue false :!label _label))
    (:MOVE_Falling
      (goto _label))
    (:MOVE_Flying
      (Variables|Default|SetMoveInput (Math|Vector2D|MakeVector2D (.x (Variables|Default|GetMoveInput)) AxisValue))
      (Pawn|Input|AddControllerPitchInput (stale Input|AxisEvents|InputAxisMouseY AxisValue)))))

(event Input|AxisEvents|InputAxisMoveRight
  (params (AxisValue :type Float%20%28single-precision%29))
  (switch Utilities|FlowControl|Switch|SwitchonEMovementMode (Variables|/Script/Engine.CharacterMovementComponent|GetMovementMode (Variables|Character|GetCharacterMovement))
    (:MOVE_Walking
      _)
    (:MOVE_Falling
      _))
  (Pawn|Input|AddMovementInput (Math|Vector|GetRightVector (Math|Rotator|MakeRotator 0.0 0.0 (.Yaw (Math|Rotator|BreakRotator (Pawn|GetControlRotation :!class /Script/Engine.Pawn))))) AxisValue false))

(fn ConstructionScript
  (|CallParentFunction))

(fn UpdateWind
  (params (DeltaTime :type Float%20%28single-precision%29))
  (Variables|Default|SetWindStrength (* DeltaTime (Math|Float|Clamp(Float) (+ (Variables|Default|GetWindStrength) (* (- (Math|Random|RandomFloat) 0.5) (* (Math|Random|RandomFloat) 1e+02))) 1e+01 1e+03))))

(fn SetFlying
  (params (IsFlying :type Boolean))
  (bind _charactermovement (Variables|Character|GetCharacterMovement))
  (bind _charactermovement_2 (Variables|Character|GetCharacterMovement))
  (if (Math|Boolean|NotEqual(Boolean) IsFlying (Utilities|Enum|Equal(Enum) (Variables|/Script/Engine.CharacterMovementComponent|GetMovementMode _charactermovement) "MOVE_Flying"))
    (if IsFlying
      (Pawn|Components|CharacterMovement|SetMovementMode _charactermovement "MOVE_Flying" 0)
      (Variables|Default|SetMovementFlyVelocity (Variables|/Script/Engine.MovementComponent|GetVelocity _charactermovement_2))
      (Variables|/Script/Engine.MovementComponent|SetVelocity _charactermovement_2 "0, 0, 0")
      (Variables|Default|SetGlideRotCurrent (Math|Rotator|CombineRotators "0.000000,90.000000,0.000000" (Transformation|GetWorldRotation (Variables|Character|GetMesh))))
      (else
        (Pawn|Components|CharacterMovement|SetMovementMode _charactermovement "MOVE_Falling" 0)
        (Physics|AddImpulse _charactermovement_2 (* (Variables|Default|GetMovementFlyVelocity) 1.5) true)
        (Transformation|SetWorldRotation (Variables|Character|GetMesh) (Math|Rotator|CombineRotators "0.000000,-90.000000,0.000000" (Variables|Default|GetGlideRotCurrent)) false false)))))

(fn UpdateGlide
  (switch Utilities|FlowControl|Switch|SwitchonEMovementMode (Variables|/Script/Engine.CharacterMovementComponent|GetMovementMode (Variables|Character|GetCharacterMovement))
    (:MOVE_Flying
      (Utilities|FlowControl|Sequence
        (:then_0
          (CallFunction|UpdateGlideRotation))
        (:then_1
          (CallFunction|UpdateGlideSpeed))
        (:then_2
          (CallFunction|UpdateGlideMovement))))))

(fn UpdateGlideRotation
  (bind _gliderotmaxpitch (Variables|Default|GetGlideRotMaxPitch))
  (Variables|Default|SetGlideRotCurrent (Math|Rotator|MakeRotator (Math|Interpolation|FInterpTo (.roll (Variables|Default|GetGlideRotCurrent)) (* (.x (Variables|Default|GetMoveInput)) (Variables|Default|GetGlideRotMaxRoll)) (Utilities|Time|GetWorldDeltaSeconds) 1.0) (Math|Interpolation|FInterpTo (.pitch (Variables|Default|GetGlideRotCurrent)) (Math|Float|Clamp(Float) (+ (* (.y (Variables|Default|GetMoveInput)) (.pitch (Variables|Default|GetGlideRotAccel)) (Utilities|Time|GetWorldDeltaSeconds)) (.pitch (Variables|Default|GetGlideRotCurrent))) (* _gliderotmaxpitch -1.0) _gliderotmaxpitch) (Utilities|Time|GetWorldDeltaSeconds) 1e+02) (Math|Interpolation|FInterpTo (.yaw (Variables|Default|GetGlideRotCurrent)) (+ (* (.x (Variables|Default|GetMoveInput)) (.yaw (Variables|Default|GetGlideRotAccel)) (Utilities|Time|GetWorldDeltaSeconds)) (.yaw (Variables|Default|GetGlideRotCurrent))) (Utilities|Time|GetWorldDeltaSeconds) 1e+01)))
  (Transformation|SetWorldRotation (Variables|Character|GetMesh) (Math|Rotator|CombineRotators "0.000000,-90.000000,90.000000" (Variables|Default|GetGlideRotCurrent)) false false))

(fn UpdateGlideSpeed
  (Variables|Default|SetGlideSpeedCurrent (Math|Float|Clamp(Float) (+ (Variables|Default|GetGlideSpeedCurrent) (* (Variables|Default|GetGlideSpeedAccel) (Utilities|Time|GetWorldDeltaSeconds) (/ (* (.pitch (Variables|Default|GetGlideRotCurrent)) -1.0) 9e+01))) 0.0 (Variables|Default|GetGlideGravityMax))))

(fn UpdateGlideMovement
  (bind _output_get (Variables|Default|SetMovementFlyVelocity (Math|Vector|Lerp(Vector) (Math|Vector|MakeVector (.x (Variables|Default|GetMovementFlyVelocity)) (+ (* (.roll (Variables|Default|GetGlideRotCurrent)) (Utilities|Time|GetWorldDeltaSeconds) 1e+01) (.y (Variables|Default|GetMovementFlyVelocity))) (Math|Float|Max(Float) (- (.z (Variables|Default|GetMovementFlyVelocity)) (* (Variables|Default|GetGlideGravityAccel) (Utilities|Time|GetWorldDeltaSeconds))) (* (Variables|Default|GetGlideGravityMax) -1.0))) (* (Math|Vector|GetForwardVector (Variables|Default|GetGlideRotCurrent)) (Variables|Default|GetGlideSpeedCurrent)) (/ (Variables|Default|GetGlideSpeedCurrent) (Variables|Default|GetGlideGravityMax)))))
  (Transformation|AddActorWorldOffset (* _output_get (Utilities|Time|GetWorldDeltaSeconds)) true))