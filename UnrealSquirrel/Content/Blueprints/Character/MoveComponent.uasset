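; Movement component for FlyingPawn that switches between walking and physics-driven gliding.
; Gliding steers with damped torques and sets velocity from a drag-based glide speed, decaying launch lift and wind.
; Wind blends global direction, storm proximity and overlapping spline windstreams, and feeds the SoundManager along with storm intensity.
; Walking moves the actor manually with simulated gravity and a ground trace; high-speed hits kill the player, and buffs modify maximum glide speed.
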(event Custom|NotifyHit
  (bind _returnvalue (Physics|GetPhysicsLinearVelocity (Variables|Default|GetMesh) "None"))
  (if (>= (Math|Vector|VectorLength _returnvalue) 1.2e+03)
    (CallFunction|KillPlayer))
  (Development|PrintString (Utilities|String|BuildString(Float) "" "HITTING STUFF AT SPEED: " (Math|Vector|VectorLength _returnvalue)) true true "(R=1.000000,G=0.002868,B=0.000000,A=1.000000)" 3.0))

(event Custom|TickMove
  (params (MoveForwardAxisValue :type Float%20%28single-precision%29) (MoveRightAxisValue :type Float%20%28single-precision%29))
  (bind _returnvalue (Utilities|Time|GetWorldDeltaSeconds))
  (bind _returnvalue_2 (Utilities|Time|GetWorldDeltaSeconds))
  (bind _returnvalue_3 (Utilities|Time|GetWorldDeltaSeconds))
  (bind _mesh (Variables|Default|GetMesh))
  (bind _parent (Variables|Default|GetParent))
  (bind _parent_2 (Variables|Default|GetParent))
  (bind _parent_3 (Variables|Default|GetParent))
  (bind _parent_4 (Variables|Default|GetParent))
  (bind _parent_5 (Variables|Default|GetParent))
  (bind _parent_6 (Variables|Default|GetParent))
  (bind _soundmanager (Variables|Default|GetSoundManager))
  (bind _parent_7 (Variables|Default|GetParent))
  (bind _movespeed (Variables|Default|GetMoveSpeed))
  (bind _skeletalmesh (Variables|Default|GetSkeletalMesh))
  (bind _skeletalmesh_2 (Variables|Default|GetSkeletalMesh))
  (bind _skeletalmesh_3 (Variables|Default|GetSkeletalMesh))
  (bind _skeletalmesh_4 (Variables|Default|GetSkeletalMesh))
  (bind _returnvalue_4 (Transformation|GetActorLocation _parent_4))
  (bind _returnvalue_5 (Transformation|GetActorLocation _parent_5))
  (bind _returnvalue_6 (Transformation|GetActorRotation _parent))
  (bind _returnvalue_7 (Transformation|GetActorRotation _parent_2))
  (bind _returnvalue_8 (Transformation|GetActorForwardVector _parent_3))
  (bind _returnvalue_9 (Transformation|GetActorRightVector _parent_3))
  (bind _returnvalue_10 (* _movespeed _returnvalue))
  (bind _springarm (Variables|/Game/Blueprints/Character/FlyingPawn.FlyingPawn_C|GetSpringArm _parent_7))
  (bind _returnvalue_11 (* _returnvalue_8 MoveForwardAxisValue))
  (bind _returnvalue_12 (* _returnvalue_9 MoveRightAxisValue))
  (bind _returnvalue_13 (+ _returnvalue_11 _returnvalue_12))
  (bind _returnvalue_14 (Math|Vector|Normalize _returnvalue_13))
  (bind _returnvalue_15 (* _returnvalue_14 _returnvalue_10))
  ;[1 1 1] Tick
  (if (not (Variables|/Game/Blueprints/Character/FlyingPawn.FlyingPawn_C|GetIsDead (Variables|Default|GetParent)))
    (Default|NotifyStormIntensityChanged (Variables|Default|GetSoundManager) (Math|Float|MapRangeClamped (+ (Math|Vector|VectorLength (- (Transformation|GetActorLocation (Variables|Default|GetStorm)) (Transformation|GetActorLocation (Variables|Default|GetParent)))) -4.7e+04) 1e+03 1e+05 1.0 0.0))
    (if (Variables|Default|GetIsFlying)
      (Default|NotifyWindIntensityChanged _soundmanager (/ (Variables|Default|GetWindSpeed) (Variables|Default|GetTargetWindSpeed)))
      (Class|PrimitiveComponent|AddTorqueinRadians (Variables|Default|GetMesh) (/ (Math|Vector|NegateVector (Class|PrimitiveComponent|GetPhysicsAngularVelocityinRadians _mesh "None")) (Variables|Default|GetTorqueDecayRate)) "None" true)
      (Development|PrintString (Utilities|String|BuildString(Float) (Utilities|String|BuildString(Vector) "" "Angular Velocity: " (Physics|GetPhysicsAngularVelocityinDegrees _mesh "None") " 
") "Current Glide Speed: " (Variables|Default|GetCurrentGlideSpeed)) true true "(R=0.140404,G=1.000000,B=0.296169,A=1.000000)" 0.01)
      (Transformation|SetActorRotation (Variables|Default|GetParent) (Math|Rotator|MakeRotator (Math|Interpolation|FInterpTo (.roll _returnvalue_6) 0.0 _returnvalue_3 1.2) (Math|Interpolation|FInterpTo (.pitch _returnvalue_6) (Math|Float|MapRangeClamped (Variables|Default|GetDragFactor) 0.0 1.0 5.0 -45.0) _returnvalue_3 1.0) (.yaw _returnvalue_6)))
      (Class|PrimitiveComponent|AddTorqueinRadians (Variables|Default|GetMesh) (Math|Vector|Lerp(Vector) "0, 0, 0" (* (Transformation|GetActorRightVector (Variables|Default|GetParent)) (* (* (Math|Float|Absolute(Float) (/ (.roll _returnvalue_6) (Variables|Default|GetMaxRoll))) -1.2) 0.8)) 1.0) "None" true)
      (Variables|Default|SetUpVelocity (Math|Interpolation|VInterpTo (Variables|Default|GetUpVelocity) "0, 0, 0" (Utilities|Time|GetWorldDeltaSeconds) 1.0))
      (Transformation|SetRelativeRotation _skeletalmesh_2 (Math|Interpolation|RInterpTo (Variables|/Script/Engine.SceneComponent|GetRelativeRotation _skeletalmesh_2) (Variables|Default|GetRelativeRotationGliding) (Utilities|Time|GetWorldDeltaSeconds) (Variables|Default|GetGlidingRotationTransitionRate)) false false)
      (Variables|Default|SetDragFactor (Math|Interpolation|FInterpTo (Variables|Default|GetDragFactor) 0.0 (Utilities|Time|GetWorldDeltaSeconds) (Variables|Default|GetDragFactorDecayRate)))
      (Transformation|SetRelativeLocation _skeletalmesh_3 (Math|Interpolation|VInterpTo (Variables|/Script/Engine.SceneComponent|GetRelativeLocation _skeletalmesh_3) "-160.000000, 0, 0" (Utilities|Time|GetWorldDeltaSeconds) (Variables|Default|GetGlidingLocationTransitionRate)) false false)
      (CallFunction|HandleWindstreams)
      (Transformation|SetRelativeRotation _springarm (Math|Interpolation|RInterpTo (Variables|/Script/Engine.SceneComponent|GetRelativeRotation _springarm) (Variables|Default|GetTargetCameraRelativeRotation) (Utilities|Time|GetWorldDeltaSeconds) 1.0) false false)
      (else
        (Default|NotifyWindIntensityChanged _soundmanager 0.0)
        (Transformation|SetRelativeRotation _skeletalmesh (Math|Interpolation|RInterpTo (Variables|/Script/Engine.SceneComponent|GetRelativeRotation _skeletalmesh) (Variables|Default|GetRelativeRotationWalking) (Utilities|Time|GetWorldDeltaSeconds) (Variables|Default|GetWalkingRotationTransitionRate)) false false)
        (Transformation|SetRelativeLocation _skeletalmesh_4 (Math|Interpolation|VInterpTo (Variables|/Script/Engine.SceneComponent|GetRelativeLocation _skeletalmesh_4) "0, 0, 0" (Utilities|Time|GetWorldDeltaSeconds) (Variables|Default|GetWalkingLocationTransitionRate)) false false)
        (Transformation|SetActorRotation _parent_2 (Math|Rotator|MakeRotator (Math|Interpolation|FInterpTo (.roll _returnvalue_7) 0.0 _returnvalue_2 8.0) (Math|Interpolation|FInterpTo (.pitch _returnvalue_7) 0.0 _returnvalue_2 1.0) (.yaw _returnvalue_7)))
        (Variables|Default|SetFallSpeed (Math|Float|Clamp(Float) (+ (Variables|Default|GetFallSpeed) (* (Variables|Default|GetGravityAccel) (Utilities|Time|GetWorldDeltaSeconds))) -1e+01 0.0))
        (bind _output_get (Variables|Default|SetVelocity (Math|Vector|MakeVector (.x _returnvalue_15) (.y _returnvalue_15) (Variables|Default|GetFallSpeed))))
        (Development|PrintString (Utilities|String|ToString(Vector) _output_get) true true "(R=0.000000,G=0.060206,B=0.262500,A=1.000000)" 0.001)
        (bind _outhit (Collision|LineTraceByChannel (+ _returnvalue_4 (Variables|Default|GetStepTraceStartOffset)) (+ (+ _returnvalue_4 (Variables|Default|GetStepTraceEndOffset)) (Variables|Default|GetVelocity)) "TraceTypeQuery3" true 0 "None" true "(R=1.000000,G=0.000000,B=0.000000,A=1.000000)" "(R=0.000000,G=1.000000,B=0.000000,A=1.000000)" 2.0))
        (Development|PrintString (Utilities|GetDisplayName (.hitactor _outhit)) true true "(R=0.000000,G=0.660000,B=1.000000,A=1.000000)" 0.01)
        (if (.bblockinghit _outhit)
          (if (<= (Math|Vector|VectorLength (- (.impactpoint _outhit) (Transformation|GetActorLocation _parent_5))) 35.0)
            (Transformation|SetActorLocation _parent_6 (Math|Vector|MakeVector (.X (Math|Vector|BreakVector (.impactpoint _outhit))) (.Y (Math|Vector|BreakVector (.impactpoint _outhit))) (.Z (Math|Vector|BreakVector (.impactpoint _outhit)))) false false)
            (Variables|Default|SetFallSpeed 0.0)
            (Variables|Default|SetUpVelocity "0, 0, 0")
            (else
              (Transformation|SetActorLocation _parent_6 (Math|Vector|MakeVector (.x _returnvalue_5) (.y _returnvalue_5) (+ (.z _returnvalue_5) (Variables|Default|GetFallSpeed))) true false)))
          (Variables|Default|SetIsOnGround true)
          (else
            (Transformation|SetActorLocation _parent_6 (Math|Vector|MakeVector (.x _returnvalue_5) (.y _returnvalue_5) (+ (.z _returnvalue_5) (Variables|Default|GetFallSpeed))) true false)
            (Transformation|SetActorLocation _parent_6 (Math|Vector|MakeVector (+ (.x _returnvalue_5) (.x (Variables|Default|GetVelocity))) (+ (.y _returnvalue_5) (.y (Variables|Default|GetVelocity))) (.z _returnvalue_5)) false false)
            (Variables|Default|SetIsOnGround false)))))))

(event Custom|MouseX
  (params (AxisValue :type Float%20%28single-precision%29))
  (bind _parent (Variables|Default|GetParent))
  (bind _returnvalue (Transformation|GetActorRotation _parent))
  ;[1 1 1] MouseX
  (if (not (Variables|/Game/Blueprints/Character/FlyingPawn.FlyingPawn_C|GetIsDead (Variables|Default|GetParent)))
    (if (Variables|Default|GetIsFlying)
      (Class|PrimitiveComponent|AddTorqueinRadians (Variables|Default|GetMesh) (* (Transformation|GetActorUpVector _parent) (* AxisValue (Variables|Default|GetTurnRateGlide))) "None" true)
      (Class|PrimitiveComponent|AddTorqueinRadians (Variables|Default|GetMesh) (* (Transformation|GetActorForwardVector (Variables|Default|GetParent)) (* AxisValue (Variables|Default|GetTurnPitchRateGlide))) "None" true)
      (else
        (Transformation|SetActorRotation (Variables|Default|GetParent) (Math|Rotator|MakeRotator (.roll _returnvalue) (.pitch _returnvalue) (+ (.yaw _returnvalue) (* AxisValue (Variables|Default|GetTurnRate)))))))))

(event Custom|MouseY
  (params (AxisValue :type Float%20%28single-precision%29))
  (bind _springarm (Variables|Default|GetSpringArm))
  (bind _maxpitch (Variables|Default|GetMaxPitch))
  (bind _lookupinverted (Variables|Default|GetLookUpInverted))
  (bind _returnvalue (Math|Conversions|ToFloat(Boolean) _lookupinverted))
  (bind _relativerotation (Variables|/Script/Engine.SceneComponent|GetRelativeRotation _springarm))
  (bind _returnvalue_2 (Math|Float|MapRangeClamped _returnvalue 1.0 0.0 -1.0 1.0))
  (bind _returnvalue_3 (* AxisValue _returnvalue_2))
  ;[1 1 1] MouseY
  (if (not (Variables|/Game/Blueprints/Character/FlyingPawn.FlyingPawn_C|GetIsDead (Variables|Default|GetParent)))
    (if (Variables|Default|GetIsFlying)
      (Class|PrimitiveComponent|AddTorqueinRadians (Variables|Default|GetMesh) (* (Transformation|GetActorRightVector (Variables|Default|GetParent)) _returnvalue_3) "None" true)
      (else
        (Transformation|SetRelativeRotation _springarm (Math|Rotator|MakeRotator (.roll _relativerotation) (+ (Math|Float|Clamp(Float) (.pitch _relativerotation) (* -1 _maxpitch) _maxpitch) (* _returnvalue_3 -1.0)) (.yaw _relativerotation)) false false)))))

(event Custom|MoveForward
  (params (AxisValue :type Float%20%28single-precision%29))
  (bind _maxglidespeed (Variables|Default|GetMaxGlideSpeed))
  (bind _upvelocity (Variables|Default|GetUpVelocity))
  ;[1 1 1] MoveForward
  (if (not (Variables|/Game/Blueprints/Character/FlyingPawn.FlyingPawn_C|GetIsDead (Variables|Default|GetParent)))
    (if (Variables|Default|GetIsFlying)
      (bind _output_get (Variables|Default|SetDragFactor (Math|Float|Clamp(Float) (+ (Variables|Default|GetDragFactor) (* AxisValue (Variables|Default|GetDragFactorRate) (Utilities|Time|GetWorldDeltaSeconds))) -1.0)))
      (Variables|Default|SetCurrentGlideSpeed (Math|Float|Clamp(Float) (* (Variables|Default|GetDragFactor) _maxglidespeed) (Variables|Default|GetMinGlideSpeed) _maxglidespeed))
      (Physics|SetPhysicsLinearVelocity (Variables|Default|GetMesh) (+ (* (Transformation|GetActorForwardVector (Variables|Default|GetParent)) (Math|Float|Clamp(Float) (* (Variables|Default|GetDragFactor) _maxglidespeed) (Variables|Default|GetMinGlideSpeed) _maxglidespeed)) (* (Variables|Default|GetWindDirection) (Variables|Default|GetWindSpeed)) _upvelocity) false "None")
      (bind _returnvalue (Physics|GetPhysicsLinearVelocity (Variables|Default|GetMesh) "None"))
      (Class|PrimitiveComponent|AddTorqueinRadians (Variables|Default|GetMesh) (* (Transformation|GetActorRightVector (Variables|Default|GetParent)) (* AxisValue (Variables|Default|GetDragFactorPitchRate))) "None" true)
      (Development|PrintString (Utilities|String|BuildString(Float) (Utilities|String|BuildString(Vector) (Utilities|String|BuildString(Vector) "" "Up Velocity: " _upvelocity " 
") "Linear Velocity: " _returnvalue " 
") "Drag Factor: " _output_get " 
") true true "(R=0.793434,G=0.078488,B=1.000000,A=1.000000)" 0.001))))

(event Custom|MoveRight
  (params (AxisValue :type Float%20%28single-precision%29))
  ;[1 1 1] MoveRight
  (if (not (Variables|/Game/Blueprints/Character/FlyingPawn.FlyingPawn_C|GetIsDead (Variables|Default|GetParent)))
    (if (Variables|Default|GetIsFlying)
      (Class|PrimitiveComponent|AddTorqueinRadians (Variables|Default|GetMesh) (* (Transformation|GetActorForwardVector (Variables|Default|GetParent)) (* AxisValue (Variables|Default|GetRollRate))) "None" true)
      (Class|PrimitiveComponent|AddTorqueinRadians (Variables|Default|GetMesh) (* (Transformation|GetActorUpVector (Variables|Default|GetParent)) (* AxisValue (Variables|Default|GetRollPitchRate))) "None" true))))

(event EventBeginPlay
  (bind _asflying_pawn (Utilities|Casting|CastToFlyingPawn (Components|GetOwner)))
  (Variables|Default|SetParent _asflying_pawn)
  (Variables|Default|SetSpringArm (Variables|/Game/Blueprints/Character/FlyingPawn.FlyingPawn_C|GetSpringArm (Variables|Default|GetParent)))
  (Variables|Default|SetMesh (Variables|/Game/Blueprints/Character/FlyingPawn.FlyingPawn_C|GetMesh (Variables|Default|GetParent)))
  (Variables|Default|SetSkeletalMesh (Variables|/Game/Blueprints/Character/FlyingPawn.FlyingPawn_C|GetSkeletalMesh (Variables|Default|GetParent)))
  (bind _storm (CallFunction|GetStorm))
  (Variables|Default|SetStorm _storm)
  (bind _soundmanager (CallFunction|GetSoundManager))
  (Variables|Default|SetSoundManager _soundmanager))

(fn HandleWindstreams
  (bind _returnvalue (Utilities|Time|GetWorldDeltaSeconds))
  (bind _affectingwindstreams (Variables|Default|GetAffectingWindstreams))
  (bind _parent (Variables|Default|GetParent))
  (bind _returnvalue_2 (Transformation|GetActorLocation _parent))
  (Variables|Default|SetTargetWindSpeed (Math|Float|MapRangeClamped (+ (Math|Vector|VectorLength (- (Transformation|GetActorLocation (Variables|Default|GetStorm)) (Transformation|GetActorLocation (Variables|Default|GetParent)))) -4.8e+04) (Variables|Default|GetMinStormDistanceWind) (Variables|Default|GetMaxStormDistanceWind) (Variables|Default|GetMaxWindspeed) (Variables|Default|GetMinWindspeed)))
  (Variables|Default|SetTargetWindDirection (Variables|Default|GetGlobalWindDirection))
  (for _array_element _affectingwindstreams
    (bind _distance (Default|FindDistanceAlongSplineClosesttoWorldLocation _array_element (Transformation|GetActorLocation (Variables|Default|GetParent))))
    (Variables|Default|SetTargetWindDirection (+ (Variables|Default|GetTargetWindDirection) (Spline|GetDirectionatDistanceAlongSpline (Variables|/Game/Blueprints/Wind/Windstream.Windstream_C|GetSpline _array_element) _distance "World")))
    (Variables|Default|SetTargetWindSpeed (+ (Variables|Default|GetTargetWindSpeed) (Variables|/Game/Blueprints/Wind/Windstream.Windstream_C|GetWindSpeed _array_element)))
    (Rendering|Debug|DrawDebugLine _returnvalue_2 (+ _returnvalue_2 (* (Variables|Default|GetWindDirection) 1e+01)) "(R=0.112741,G=0.412059,B=0.572917,A=1.000000)" 1.5 4.0)
    (Rendering|Debug|DrawDebugLine (Spline|GetLocationatDistanceAlongSpline (Variables|/Game/Blueprints/Wind/Windstream.Windstream_C|GetSpline _array_element) _distance "World") (+ (Spline|GetLocationatDistanceAlongSpline (Variables|/Game/Blueprints/Wind/Windstream.Windstream_C|GetSpline _array_element) _distance "World") (* (Spline|GetDirectionatDistanceAlongSpline (Variables|/Game/Blueprints/Wind/Windstream.Windstream_C|GetSpline _array_element) _distance "World") 1e+01)) "(R=0.572917,G=0.148500,B=0.551241,A=1.000000)" 1.5 4e+01))
  (Default|NotifyWindStream (Variables|Default|GetSoundManager) (!= (Utilities|Array|Length _affectingwindstreams) 0))
  (Variables|Default|SetWindDirection (Math|Interpolation|VInterpTo (Variables|Default|GetWindDirection) (Math|Vector|Normalize (Variables|Default|GetTargetWindDirection)) _returnvalue 1.0))
  (Variables|Default|SetWindSpeed (Math|Interpolation|FInterpTo (Variables|Default|GetWindSpeed) (Variables|Default|GetTargetWindSpeed) _returnvalue 0.5))
  (Development|PrintString (Utilities|String|BuildString(Float) (Utilities|String|BuildString(Float) (Utilities|String|BuildString(Vector) (Utilities|String|BuildString(Vector) "" "Current Wind Dir: " (Variables|Default|GetWindDirection) " 
") "; Target Wind Dir: " (Math|Vector|Normalize (Variables|Default|GetTargetWindDirection)) " 
") "Current Wind Speed: " (Variables|Default|GetWindSpeed) " 
") "Target Wind Speed: " (Variables|Default|GetTargetWindSpeed)) true true "(R=0.000000,G=0.000000,B=0.000000,A=1.000000)" 0.001))

(fn ToggleFlying
  (params (NewIsFlying :type Boolean))
  (if (not NewIsFlying)
    (Variables|Default|SetIsFlying false)
    (Class|PrimitiveComponent|SetConstraintMode (Variables|Default|GetMesh) "SixDOF")
    (Physics|SetSimulatePhysics (Variables|Default|GetMesh) false)
    (Variables|Default|SetTargetActorRotation (Math|Rotator|MakeRotator 0.0 0.0 (.yaw (Transformation|GetActorRotation (Variables|Default|GetParent)))))
    (Collision|SetCollisionProfileName (Variables|Default|GetMesh) "Pawn" true :!class /Script/Engine.PrimitiveComponent)
    (Variables|Default|SetDragFactor 0.0)
    (Variables|Default|SetIsOnGround false)
    (bind _soundmanager (CallFunction|GetSoundManager))
    (Default|NotifyFlying _soundmanager false)
    (else
      (Variables|Default|SetIsFlying true)
      (Class|PrimitiveComponent|SetConstraintMode (Variables|Default|GetMesh) "SixDOF")
      (Physics|SetSimulatePhysics (Variables|Default|GetMesh) true)
      (Collision|SetCollisionProfileName (Variables|Default|GetMesh) "PhysicsActor" true :!class /Script/Engine.PrimitiveComponent)
      (if (not (!= (Math|Vector|VectorLength (Variables|Default|GetUpVelocity)) 0.0))
        (Variables|Default|SetUpVelocity "0, 0,350.000000")
        (Variables|Default|SetTargetCameraRelativeRotation "0, 0, 0")
        (Variables|Default|SetDragFactor 0.0)
        (Variables|Default|SetIsOnGround false)
        (bind _soundmanager_2 (CallFunction|GetSoundManager))
        (Default|NotifyFlying _soundmanager_2 true)))))

(fn PrintRotations
  (Development|PrintString (Class|KismetStringLibrary|BuildStringRotator (Class|KismetStringLibrary|BuildStringRotator (Class|KismetStringLibrary|BuildStringRotator (Class|KismetStringLibrary|BuildStringRotator "" "Mesh: " (Transformation|GetWorldRotation (Variables|Default|GetMesh)) " 
") "SpringArm: " (Transformation|GetWorldRotation (Variables|Default|GetSpringArm)) " 
") "SkelMesh: " (Transformation|GetWorldRotation (Variables|Default|GetSkeletalMesh)) " 
") "Capsule: " (Transformation|GetWorldRotation (Variables|/Game/Blueprints/Character/FlyingPawn.FlyingPawn_C|GetCapsule (Variables|Default|GetParent))) " 
") true true "(R=0.000000,G=0.660000,B=1.000000,A=1.000000)" 5.0))

(fn PrintLocations
  (Development|PrintString (Utilities|String|BuildString(Vector) (Utilities|String|BuildString(Vector) (Utilities|String|BuildString(Vector) (Utilities|String|BuildString(Vector) "" "Mesh: " (Variables|/Script/Engine.SceneComponent|GetRelativeLocation (Variables|Default|GetMesh)) " 
") "SpringArm: " (Variables|/Script/Engine.SceneComponent|GetRelativeLocation (Variables|Default|GetSpringArm)) " 
") "SkelMesh: " (Variables|/Script/Engine.SceneComponent|GetRelativeLocation (Variables|Default|GetSkeletalMesh)) " 
") "Capsule: " (Variables|/Script/Engine.SceneComponent|GetRelativeLocation (Variables|/Game/Blueprints/Character/FlyingPawn.FlyingPawn_C|GetCapsule (Variables|Default|GetParent))) " 
") true true "(R=0.000000,G=0.660000,B=1.000000,A=1.000000)" 5.0))

(fn AddBuff
  (params (Buff :type Buff%20Structure))
  (switch Utilities|FlowControl|Switch|SwitchonEBuffType (.type Buff)
    (:NewEnumerator0
      (switch Utilities|FlowControl|Switch|SwitchonEBuffOperation (.operation Buff)
        (:NewEnumerator0
          (Variables|Default|SetMaxGlideSpeed (+ (Variables|Default|GetMaxGlideSpeed) (.value Buff))))
        (:NewEnumerator1
          (Variables|Default|SetMaxGlideSpeed (* (Variables|Default|GetMaxGlideSpeed) (.value Buff))))
        (:NewEnumerator2
          (Variables|Default|SetMaxGlideSpeed (.value Buff)))))))