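; CharacterNPC is a character Blueprint for NPCs that move along an assigned path and can be talked to.
; After each successful AI move it waits briefly at random, then asks AssignedPath for the next target.
; Interaction starts the dialogue camera and a chat bubble, while separate events stop it facing the player or restore its movement.
; Outline highlighting toggles custom depth and stencil on the mesh.
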(event Custom|AIMoveTo
  (params (targetLocation :type Vector))
  (if (Variables|Default|GetShouldMove)
    (bind _movementresult (AI|AIMoveTo self targetLocation 0 5.0 false)
      (:OnSuccess
        (CallFunction|WaitatTargetedLocation))
      (:OnFail
        (Development|PrintString (Utilities|String|EnumtoString _movementresult) true true "(R=1.000000,G=0.031556,B=0.000000,A=1.000000)" 5.0)))))

(event Custom|InteracedWith
  (Default|InitDialogueCamera (CallFunction|GetDialogueCamera) self)
  (CallFunction|SpawnChatBubble self))

(event Custom|StopMovingLookAtPlayer
  (Transformation|SetActorRotation (Math|Rotator|FindLookatRotation (Transformation|GetActorLocation self) (Transformation|GetActorLocation (CallFunction|GetPlayer))))
  (CallFunction|CancelMovement))

(event Custom|WaitAtTargetedLocation
  (bind _assignedpath (Variables|Default|GetAssignedPath))
  (Utilities|FlowControl|Delay (Math|Random|RandomFloatinRange 1.0 2.0))
  (Default|ReachedTargetedLocation _assignedpath)
  (Default|FindTargetLocation _assignedpath))

(event Custom|RestartMovement
  (Variables|/Script/Engine.CharacterMovementComponent|SetMaxWalkSpeed (Variables|Character|GetCharacterMovement) (Variables|Default|GetInitialMovementSpeed))
  (Variables|Default|SetShouldMove true))

(event Custom|CancelMovement
  (Variables|/Script/Engine.CharacterMovementComponent|SetMaxWalkSpeed (Variables|Character|GetCharacterMovement) 0.0)
  (Variables|Default|SetShouldMove false))

(event Custom|EnableOutline
  (bind _mesh (Variables|Character|GetMesh))
  (Rendering|SetRenderCustomDepth _mesh true)
  (Rendering|SetCustomDepthStencilValue _mesh 2))

(event Custom|DisableOutline
  (bind _mesh (Variables|Character|GetMesh))
  (Rendering|SetCustomDepthStencilValue _mesh 0)
  (Rendering|SetRenderCustomDepth _mesh false))

(event EventBeginPlay
  (Variables|Default|SetInitialMovementSpeed (Variables|/Script/Engine.CharacterMovementComponent|GetMaxWalkSpeed (Variables|Character|GetCharacterMovement))))

(fn ConstructionScript
  (|CallParentFunction))