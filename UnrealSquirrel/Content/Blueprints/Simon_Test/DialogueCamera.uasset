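; DialogueCamera is an actor that frames a dialogue between the player and an NPC by becoming the player's view target.
; On initialization it stores both characters, moves to the midpoint between them and rotates to match the player-to-NPC direction.
; It then eases the player controller's view over to itself and tells the NPC to stop moving and look at the player.
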(event Custom|InitDialogueCamera
  (params (characterNPC :type Character%20NPC%20Object%20Reference))
  (Variables|Default|SetPlayer (CallFunction|GetPlayer))
  (Variables|Default|SetNPCDialogueTarget characterNPC)
  (CallFunction|GetCameraPositionandLookat))

(event Custom|GetCameraPositionAndLookAt
  (bind _output_get (Variables|Default|SetCameraLocation (/ (+ (Transformation|GetActorLocation (CallFunction|GetPlayer)) (Transformation|GetActorLocation (Variables|Default|GetNPCDialogueTarget))) 2)))
  (Transformation|SetActorRotation (Math|Rotator|FindLookatRotation (Transformation|GetActorLocation (Variables|Default|GetPlayer)) (Transformation|GetActorLocation (Variables|Default|GetNPCDialogueTarget))))
  (Transformation|SetActorLocation _output_get false false)
  (CallFunction|SetCamera)
  (Default|StopMovingLookatPlayer (Variables|Default|GetNPCDialogueTarget)))

(event Custom|SetCamera
  (bind _asplayer_controller (Utilities|Casting|CastToPlayerController (Pawn|GetController (Variables|Default|GetPlayer))))
  (Game|Player|SetViewTargetwithBlend _asplayer_controller self 1.0 "VTBlend_EaseInOut" 0.7 false))

(event EventBeginPlay)

(event Collision|EventActorBeginOverlap
  (params (OtherActor :type Actor%20Object%20Reference)))

(event EventTick
  (params (DeltaSeconds :type Float%20%28single-precision%29)))

(fn ConstructionScript)