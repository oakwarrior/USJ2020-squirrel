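; Coin pickup actor for the flying pawn that awards a coin and a movement buff.
; A Rotation timeline restarts itself on finish to keep the coin spinning in yaw.
; On sphere overlap with a FlyingPawn it increments that pawn's coins, plays a sound and adds the buff to the player's MoveComponent.
; The coin is hidden rather than destroyed, with a flag blocking repeat pickups.
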(event OnComponentBeginOverlap(Sphere)
  (params (OverlappedComponent :type Primitive%20Component%20Object%20Reference) (OtherActor :type Actor%20Object%20Reference) (OtherComp :type Primitive%20Component%20Object%20Reference) (OtherBodyIndex :type Integer) (bFromSweep :type Boolean) (SweepResult :type Hit%20Result%20Structure%20%28by%20ref%29))
  (if (not (Variables|Default|GetIsPickedUp))
    (bind _asflying_pawn (Utilities|Casting|CastToFlyingPawn OtherActor))
    (Default|IncrementCoins _asflying_pawn)
    (CallFunction|PlaySFX "NewEnumerator0")
    (Rendering|SetActorHiddenInGame true)
    (Variables|Default|SetIsPickedUp true)
    (Default|AddBuff (Variables|/Game/Blueprints/Character/FlyingPawn.FlyingPawn_C|GetMoveComponent (CallFunction|GetPlayer)) (Variables|Default|GetBuff))))

(event Custom|StartRotation
  (bind _newtrack_0 (Timeline|Rotation PlayFromStart)
    (:Update
      (Transformation|SetActorRotation (Math|Rotator|MakeRotator 0.0 0.0 _newtrack_0)))
    (:Finished
      (CallFunction|StartRotation))))

(event EventBeginPlay
  (CallFunction|StartRotation))

(fn ConstructionScript)