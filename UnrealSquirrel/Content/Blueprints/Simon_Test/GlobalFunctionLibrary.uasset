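; Blueprint function library of global helpers for reaching key level actors from anywhere in the game.
; GetDialogueCamera and GetPlayer return the first DialogueCamera and CharacterPlayer found with GetAllActorsOfClass.
; PlaySFX finds the first SoundManager the same way and passes it a sound type to play.
; Each call searches the level anew and takes index zero without checking that an actor exists.
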(fn GetDialogueCamera
  (bind _outactors (Actor|GetAllActorsOfClass 0 "/Game/Blueprints/Simon_Test/DialogueCamera.DialogueCamera_C"))
  (return (Utilities|Array|Get(acopy) _outactors)))

(fn GetPlayer
  (bind _outactors (Actor|GetAllActorsOfClass 0 "/Game/Blueprints/Character/CharacterPlayer.CharacterPlayer_C"))
  (return (Utilities|Array|Get(acopy) _outactors)))

(fn PlaySFX
  (params (SoundType :type SoundTypes%20Enum :default "NewEnumerator0"))
  (bind _outactors (Actor|GetAllActorsOfClass 0 "/Game/Blueprints/Simon_Test/SoundManager.SoundManager_C"))
  (Default|PlaySound (Utilities|Array|Get(acopy) _outactors) SoundType))