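; Spline path actor that serves as a back-and-forth patrol route for one assigned NPC.
; On BeginPlay it sends the NPC to the targeted spline point and registers itself as that NPC's path.
; ReachedTargetedLocation steps the point index and flips direction at either end, but does not issue the next move.
; FindTargetLocation resolves the point's world position and issues the AI move, while GetControllerNPC caches the NPC's controller.
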(event Custom|FindTargetLocation
  (Variables|Default|SetTargetLocation (Spline|GetLocationatSplinePoint (Variables|Default|GetNPCPathSpline) (Variables|Default|GettargetedSplinePoint) "World"))
  (Default|AIMoveto (Variables|Default|GetAsignedNPC) (Variables|Default|GetTargetLocation)))

(event Custom|ReachedTargetedLocation
  (bind _npcpathspline (Variables|Default|GetNPCPathSpline))
  (bind _returnvalue (Spline|GetNumberOfSplinePoints _npcpathspline))
  (if (>= _returnvalue (Variables|Default|GettargetedSplinePoint))
    (Variables|Default|SettargetedSplinePoint (+ (Variables|Default|GettargetedSplinePoint) (* 1 (Variables|Default|GetPathDirection))))
    (if (>= (Variables|Default|GettargetedSplinePoint) _returnvalue)
      (Variables|Default|SetPathDirection -1)
      (elif (<= (Variables|Default|GettargetedSplinePoint) 0)
        (Variables|Default|SetPathDirection 1)))))

(event Custom|GetControllerNPC
  (bind _ascontroller_npc (Utilities|Casting|CastToControllerNPC (Pawn|GetController (Variables|Default|GetAsignedNPC))))
  (Variables|Default|SetControllerNPC _ascontroller_npc))

(event EventBeginPlay
  (bind _asignednpc (Variables|Default|GetAsignedNPC))
  (CallFunction|FindTargetLocation)
  (Default|AIMoveto _asignednpc (Variables|Default|GetTargetLocation))
  (Variables|/Game/Blueprints/Character/CharacterNPC.CharacterNPC_C|SetAssignedPath _asignednpc self))

(fn ConstructionScript)