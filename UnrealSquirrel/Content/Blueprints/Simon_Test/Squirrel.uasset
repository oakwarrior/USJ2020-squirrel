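; Squirrel is a test Blueprint, apparently player-controlled, that drives the start screen and dialogue UI and tracks a coin count.
; BeginPlay shows a StartGame widget, and any key press calls its start function and completes the text of any open dialogue.
; Interact lazily creates and reuses a DialogueWidget, opening it with hardcoded test text.
; IncrementCoins adds one to Points.
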(event Custom|AddDialogueBox
  (Utilities|IsValid (Variables|Default|GetDialogueBox)
    (:Is%20Valid
      (Default|OpenDialogueWidget (Variables|Default|GetDialogueBox) "This text is for testing! and testing is what i'll DO!"))
    (:Is%20Not%20Valid
      (bind _returnvalue (UserInterface|CreateWidget "/Game/Blueprints/Simon_Test/DialogueWidget.DialogueWidget_C"))
      (Variables|Default|SetDialogueBox _returnvalue)
      (UserInterface|Viewport|AddtoViewport _returnvalue 0)
      (Default|OpenDialogueWidget _returnvalue "This text is for testing! and testing is what i'll DO!"))))

(event Custom|IncrementCoins
  (Math|Integer|IncrementInt (Variables|Default|Getpoints)))

(event EventBeginPlay
  (bind _returnvalue (UserInterface|CreateWidget "/Game/Blueprints/Simon_Test/StartGame.StartGame_C"))
  (UserInterface|Viewport|AddtoViewport _returnvalue 0)
  (Variables|Default|SetStartScreen _returnvalue))

(event Input|ActionEvents|InputActionAnyInputKey
  (params (Key :type Key%20Structure :default "None"))
  (bind _dialoguebox (Variables|Default|GetDialogueBox))
  (:Pressed
    (Default|StartGame (Variables|Default|GetStartScreen))
    (Utilities|IsValid _dialoguebox
      (:Is%20Valid
        (Default|CompleteText _dialoguebox)))))

(event Input|ActionEvents|InputActionInteract
  (params (Key :type Key%20Structure :default "None"))
  (:Pressed
    (CallFunction|AddDialogueBox)))

(fn ConstructionScript)