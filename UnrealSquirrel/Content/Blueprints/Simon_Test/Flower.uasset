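; Flower is a decorative actor that picks its look from seven flower material instances.
; The construction script applies the same material to both of its plane meshes, Plane and Plane1.
; The Custom flag selects the material by Index; otherwise a random one is rolled whenever construction runs.
; The event graph has no active logic.
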(event EventBeginPlay)

(event Collision|EventActorBeginOverlap
  (params (OtherActor :type Actor%20Object%20Reference)))

(event EventTick
  (params (DeltaSeconds :type Float%20%28single-precision%29)))

(fn ConstructionScript
  (if (Variables|Default|Getcustom)
    (Rendering|Material|SetMaterial (Variables|Default|GetPlane) 0 (Utilities|Select :Index (Variables|Default|GetIndex) :Option%200 "/Game/Art/Materials/Flower_Inst.Flower_Inst" :Option%201 "/Game/Art/Materials/Flower_Inst1.Flower_Inst1" :Option%202 "/Game/Art/Materials/Flower_Inst2.Flower_Inst2" :Option%203 "/Game/Art/Materials/Flower_Inst3.Flower_Inst3" :Option%204 "/Game/Art/Materials/Flower_Inst4.Flower_Inst4" :Option%205 "/Game/Art/Materials/Flower_Inst5.Flower_Inst5" :Option%206 "/Game/Art/Materials/Flower_Inst6.Flower_Inst6"))
    (else
      (Rendering|Material|SetMaterial (Variables|Default|GetPlane) 0 (Utilities|Select :Index (Math|Random|RandomIntegerinRange 0 6) :Option%200 "/Game/Art/Materials/Flower_Inst.Flower_Inst" :Option%201 "/Game/Art/Materials/Flower_Inst1.Flower_Inst1" :Option%202 "/Game/Art/Materials/Flower_Inst2.Flower_Inst2" :Option%203 "/Game/Art/Materials/Flower_Inst3.Flower_Inst3" :Option%204 "/Game/Art/Materials/Flower_Inst4.Flower_Inst4" :Option%205 "/Game/Art/Materials/Flower_Inst5.Flower_Inst5" :Option%206 "/Game/Art/Materials/Flower_Inst6.Flower_Inst6")))))