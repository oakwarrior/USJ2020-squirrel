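; SoundManager is a test-folder Blueprint that centralizes game audio, starting FMOD music on BeginPlay and exposing events for gameplay to call.
; PlaySound switches on a sound-type enum to per-sound events, though only the coin pickup calls a 2D playback and the rest are empty stubs.
; Notify events feed flying, storm, wind intensity and windstream state into FMOD parameters on music, storm and wind components for adaptive audio.
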(event Custom|PlaySound
  (params (SoundType :type SoundTypes%20Enum :default "NewEnumerator0"))
  (switch Utilities|FlowControl|Switch|SwitchonSoundTypes SoundType
    (:NewEnumerator0
      (CallFunction|PlayGetCoin))
    (:NewEnumerator1
      (CallFunction|PlayFootstep))
    (:NewEnumerator2
      (CallFunction|PlayInteract))
    (:NewEnumerator3
      (CallFunction|PlayStartGame))
    (:NewEnumerator4
      (CallFunction|123))
    (:NewEnumerator5
      (CallFunction|PlayLetterAdded))))

(event Custom|PlayGetCoin
  (Audio|PlaySound2D 0 1.0 1.0 0.0 0 0))

(event Custom|NotifyWindStream
  (params (IsInWindStream :type Boolean))
  (Class|FMODAudioComponent|SetParameter (Variables|Default|GetFMODWind) "Windstream" (Math|Conversions|ToFloat(Boolean) IsInWindStream)))

(event Custom|NotifyWindIntensityChanged
  (params (Intensity :type Float%20%28single-precision%29))
  (Class|FMODAudioComponent|SetParameter (Variables|Default|GetFMODWind) "Fly Speed" Intensity))

(event Custom|PlayInteract)

(event Custom|PlayFootstep)

(event Custom|PlayLetterAdded)

(event Custom|PlayStartGame)

(event Custom|123)

(event Custom|NotifyFlying
  (params (IsFlying :type Boolean))
  (Class|FMODAudioComponent|SetParameter (Variables|Default|GetFMODMusic) "Flying" (Math|Conversions|ToFloat(Boolean) IsFlying)))

(event Custom|NotifyStormIntensityChanged
  (params (Storm :type Float%20%28single-precision%29))
  (Class|FMODAudioComponent|SetParameter (Variables|Default|GetFMODMusic) "Storm" Storm)
  (Class|FMODAudioComponent|SetParameter (Variables|Default|GetFMODStormSFX) "Storm" Storm))

(event EventBeginPlay
  (Class|FMODAudioComponent|Play (Variables|Default|GetFMODMusic)))

(fn ConstructionScript)