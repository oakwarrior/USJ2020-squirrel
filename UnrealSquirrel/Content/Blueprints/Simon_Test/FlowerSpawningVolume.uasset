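; A volume that scatters a set number of Flower actors across world-static surfaces within its box bounds.
; On BeginPlay or SpawnFlowers, it line-traces downward through random box points and spawns at each hit location with random yaw and per-axis scale, without checking for a hit.
; Spawned flowers are kept in an array, which DeleteFlowers destroys and clears.
; Random selection from TypesOfFlowersToSpawn is left unconnected.
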(event Custom|DeleteFlowers
  (for _array_element (Variables|Default|GetFlowers)
    (Actor|DestroyActor _array_element))
  (Utilities|Array|Clear (Variables|Default|GetFlowers)))

(event Custom|SpawnFlowers
  (bind _returnvalue (Math|Random|RandomFloatinRange 0.8 1.2))
  (bind _box (Variables|Default|GetBox))
  (bind (_origin _boxextent) (Collision|GetComponentBounds _box))
  (bind _returnvalue_2 (Math|Random|RandomPointinBoundingBox _origin _boxextent))
  (for _index (range 0 (Variables|Default|GetAmountOfFlowersToSpawn))
    (bind _outhit (Collision|LineTraceForObjects (+ _returnvalue_2 "0, 0,99999.000000") (+ _returnvalue_2 "0, 0,-99999.000000") (Utilities|Array|MakeArray "ObjectTypeQuery1") false 0 "ForDuration"))
    (Game|SpawnActorfromClass "/Game/Blueprints/Simon_Test/Flower.Flower_C" (Math|Transform|MakeTransform (.Location (Collision|BreakHitResult _outhit)) (Math|Rotator|MakeRotator 0.0 0.0 (Math|Random|RandomFloatinRange 0.0 3.6e+02)) (Math|Vector|MakeVector _returnvalue _returnvalue _returnvalue)) "Undefined" 0 0)
    (Utilities|Array|Add (Variables|Default|GetFlowers) 0)))

(event EventBeginPlay
  (bind _returnvalue (Math|Random|RandomFloatinRange 0.8 1.2))
  (bind _box (Variables|Default|GetBox))
  (bind (_origin _boxextent) (Collision|GetComponentBounds _box))
  (bind _returnvalue_2 (Math|Random|RandomPointinBoundingBox _origin _boxextent))
  (for _index (range 0 (Variables|Default|GetAmountOfFlowersToSpawn))
    (bind _outhit (Collision|LineTraceForObjects (+ _returnvalue_2 "0, 0,99999.000000") (+ _returnvalue_2 "0, 0,-99999.000000") (Utilities|Array|MakeArray "ObjectTypeQuery1") false 0 "ForDuration"))
    (Game|SpawnActorfromClass "/Game/Blueprints/Simon_Test/Flower.Flower_C" (Math|Transform|MakeTransform (.Location (Collision|BreakHitResult _outhit)) (Math|Rotator|MakeRotator 0.0 0.0 (Math|Random|RandomFloatinRange 0.0 3.6e+02)) (Math|Vector|MakeVector _returnvalue _returnvalue _returnvalue)) "Undefined" 0 0)
    (Utilities|Array|Add (Variables|Default|GetFlowers) 0)))

(event Collision|EventActorBeginOverlap
  (params (OtherActor :type Actor%20Object%20Reference)))

(event EventTick
  (params (DeltaSeconds :type Float%20%28single-precision%29)))

(fn ConstructionScript)